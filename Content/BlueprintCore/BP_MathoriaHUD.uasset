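; BP_MathoriaHUD is the front-end Blueprint that shows the splash screen and routes the player on tap-to-play.
; On BeginPlay it adds the splash widget to the viewport and binds its tap button.
; On tap, a signed-in, email-verified user whose player state passes its OnSplashScreen check gets the splash collapsed and the overlay opened.
; Otherwise the authentication widget opens above the splash, with both follow-up widgets receiving a splash reference.
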(event Custom|OnClicked_Event
  (bind _returnvalue (Class|AuthMiscLibrary|CurrentUser))
  (Utilities|IsValid _returnvalue
    (:Is%20Valid
      (if (Class|User|IsEmailVerified _returnvalue)
        (bind _asbp_mathoria_player_state (Utilities|Casting|CastToBP_MathoriaPlayerState (Game|GetPlayerState 0)))
        (bind _returnvalue_2 (Class|MathoriaPlayerState|OnSplashScreen _asbp_mathoria_player_state))
        (if _returnvalue_2
          (Widget|SetVisibility (Variables|Default|GetSplashScreenRef) "Collapsed")
          (bind _returnvalue_3 (UserInterface|CreateWidget "/Game/Widgets/WBP_Overlay.WBP_Overlay_C" (Game|GetPlayerController 0) (Variables|Default|GetSplashScreenRef)))
          (UserInterface|Viewport|AddtoViewport _returnvalue_3 4)
          (else
            (bind _returnvalue_4 (UserInterface|CreateWidget "/Game/Widgets/WBP_Authenticate.WBP_Authenticate_C" (Game|GetPlayerController 0) (Variables|Default|GetSplashScreenRef) :!label _label))
            (UserInterface|Viewport|AddtoViewport _returnvalue_4 3)))
        (else
          (goto _label))))
    (:Is%20Not%20Valid
      (goto _label))))

(event EventBeginPlay
  (bind _returnvalue (UserInterface|CreateWidget "/Game/Widgets/WBP_SplashSreen.WBP_SplashSreen_C" (Game|GetPlayerController 0)))
  (UserInterface|Viewport|AddtoViewport _returnvalue 2)
  (bind _output_get (Variables|Default|SetSplashScreenRef _returnvalue))
  (EventDispatchers|AssignOnClicked (Variables|/Game/Widgets/WBP_SplashSreen.WBP_SplashSreen_C|GetTapToPlayButton _output_get) (delegate Custom|OnClicked_Event)))

(event Collision|EventActorBeginOverlap
  (params (OtherActor :type Actor%20Object%20Reference)))

(event EventTick
  (params (DeltaSeconds :type Float%20%28single-precision%29)))

(fn ConstructionScript)